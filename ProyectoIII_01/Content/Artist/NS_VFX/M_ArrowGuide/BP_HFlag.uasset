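; BP_HFlag is a flag actor in the arrow guide VFX folder that animates vertically and rotates when its box is overlapped.
; The Loop timeline offsets the actor's Z from its start location, alternating endlessly with a second timeline that only spaces out replays.
; Any box overlap plays Timeline_0, adding yaw to the Flag's captured world rotation and applying the result as relative rotation.
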(event OnComponentBeginOverlap(Box)
  (params (OverlappedComponent :type Primitive%20Component%20Object%20Reference) (OtherActor :type Actor%20Object%20Reference) (OtherComp :type Primitive%20Component%20Object%20Reference) (OtherBodyIndex :type Integer) (bFromSweep :type Boolean) (SweepResult :type Hit%20Result%20Structure%20%28by%20ref%29))
  (bind _flag (Variables|Default|GetFlag))
  (Variables|Default|SetStart_rotation (Transformation|GetWorldRotation _flag))
  (bind _loop (Timeline|Timeline_0 PlayFromStart)
    (:Update
      (Transformation|SetRelativeRotation _flag (Math|Rotator|MakeRotator (.roll (Variables|Default|GetStart_rotation)) (.pitch (Variables|Default|GetStart_rotation)) (+ _loop (.yaw (Variables|Default|GetStart_rotation)))) false false))))

(event EventBeginPlay
  (Variables|Default|SetStart_location (Transformation|GetActorLocation))
  (bind _loop (Timeline|Loop PlayFromStart)
    (:Update
      (Transformation|SetActorLocation (Math|Vector|MakeVector (.x (Variables|Default|GetStart_location)) (.y (Variables|Default|GetStart_location)) (+ _loop (.z (Variables|Default|GetStart_location)))) false false))
    (:Finished
      (Timeline|Timeline PlayFromStart
        (:Finished
          (Timeline|Loop PlayFromStart))))))

(event Collision|EventActorBeginOverlap
  (params (OtherActor :type Actor%20Object%20Reference)))

(event EventTick
  (params (DeltaSeconds :type Float%20%28single-precision%29)))

(fn ConstructionScript)