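; Boost panel for the player ship that plays a sound on overlap and raises the ship's Force within a clamped range.
; The ship's BoostPanel flag blocks repeat boosts while speed lines run for two seconds; Force is not restored here.
; Timed Entering and Stopping flags make Tick step the boost post-process blend weight up, then down, at a frame-rate-dependent rate.
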(event OnComponentBeginOverlap(Box)
  (params (OverlappedComponent :type Primitive%20Component%20Object%20Reference) (OtherActor :type Actor%20Object%20Reference) (OtherComp :type Primitive%20Component%20Object%20Reference) (OtherBodyIndex :type Integer) (bFromSweep :type Boolean) (SweepResult :type Hit%20Result%20Structure%20%28by%20ref%29))
  (bind _returnvalue (Game|Player|GetPlayerPawn 0))
  (bind _asship (Utilities|Casting|CastToShip _returnvalue))
  (bind _speedlines_vfx (Variables|/Game/Devs/Ship/Ship.Ship_C|GetSpeedLines_VFX _asship))
  (if (== OtherActor (Variables|Default|GetShip_SM))
    (Audio|PlaySound2D "/Game/Devs/Circuit/BoostBarrierSound.BoostBarrierSound" 1.0 1.0 0.0 0 0)
    (if (not (Variables|/Game/Devs/Ship/Ship.Ship_C|GetBoostPanel (.AsShip (Utilities|Casting|CastToShip (Game|Player|GetPlayerPawn 0)))))
      (Utilities|FlowControl|Sequence
        (:then_0
          (Variables|/Game/Devs/Ship/Ship.Ship_C|SetBoostPanel _asship true)
          (Variables|/Game/Devs/Ship/Ship.Ship_C|Setforce _asship (Math|Float|Clamp(Float) (* (Variables|/Game/Devs/Ship/Ship.Ship_C|Getforce _asship) 1.2) 1e+05 3e+05))
          (Components|Activation|Activate _speedlines_vfx false)
          (Utilities|FlowControl|Delay 2.0)
          (Variables|/Game/Devs/Ship/Ship.Ship_C|SetBoostPanel _asship false)
          (Components|Activation|Deactivate _speedlines_vfx))
        (:then_1
          ;[0.15 0.15 0.15 0.5] Enter_visibility
          (Variables|Default|SetEntering true)
          (Utilities|FlowControl|Delay 0.5)
          (Variables|Default|SetEntering false))
        (:then_2
          ;[0.15 0.15 0.15 0.5] Exit_visibility
          (Utilities|FlowControl|Delay 1.0)
          (Variables|Default|SetStopping true)
          (Utilities|FlowControl|Delay 0.5)
          (Variables|Default|SetStopping false))))))

(event EventBeginPlay
  (Variables|/Script/Engine.PostProcessVolume|SetBlendWeight (Variables|Default|GetPP_Boost) 0.0)
  (Variables|/Script/Engine.PostProcessVolume|SetBlendWeight (Variables|Default|GetPP_Debuff) 0.0)
  (Variables|Default|SetShip_SM (Game|Player|GetPlayerPawn 0)))

(event Collision|EventActorBeginOverlap
  (params (OtherActor :type Actor%20Object%20Reference)))

(event EventTick
  (params (DeltaSeconds :type Float%20%28single-precision%29))
  (Utilities|FlowControl|Sequence
    (:then_0
      (if (Variables|Default|GetEntering)
        (bind _output_get (Variables|/Script/Engine.PostProcessVolume|SetBlendWeight (Variables|Default|GetPP_Boost) (+ (Variables|Default|GetPP_Visibility) 0.1)))
        (Variables|Default|SetPP_Visibility _output_get)))
    (:then_1
      ;[0.15 0.15 0.15 0.5] Visibility_fade
      (if (Variables|Default|GetStopping)
        (bind _output_get_2 (Variables|/Script/Engine.PostProcessVolume|SetBlendWeight (Variables|Default|GetPP_Boost) (- (Variables|Default|GetPP_Visibility) 0.1)))
        (Variables|Default|SetPP_Visibility _output_get_2)))))

(fn ConstructionScript)