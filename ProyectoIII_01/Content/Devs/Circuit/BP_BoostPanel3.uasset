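; BP_BoostPanel3 is a boost panel actor for the ship that hands barrier overlaps to its BoostBarrierComponent.
; BeginPlay zeroes the boost and debuff post-process weights and caches the player pawn.
; Tick can fade the boost post-process in or out through Entering and Stopping flags.
; Those flags are set only in disconnected older logic, which also held the sound, timed force boost and speed-line VFX.
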(event OnComponentBeginOverlap(Barrier_1_Sides2)
  (params (OverlappedComponent :type Primitive%20Component%20Object%20Reference) (OtherActor :type Actor%20Object%20Reference) (OtherComp :type Primitive%20Component%20Object%20Reference) (OtherBodyIndex :type Integer) (bFromSweep :type Boolean) (SweepResult :type Hit%20Result%20Structure%20%28by%20ref%29))
  (Default|OnOverlap (Variables|Default|GetBoostBarrierComponent) OtherActor))

(event EventBeginPlay
  (Variables|/Script/Engine.PostProcessVolume|SetBlendWeight (Variables|Default|GetPP_Boost) 0.0)
  (Variables|/Script/Engine.PostProcessVolume|SetBlendWeight (Variables|Default|GetPP_Debuff) 0.0)
  (Variables|Default|SetShip_SM (Game|Player|GetPlayerPawn 0)))

(event EventTick
  (params (DeltaSeconds :type Float%20%28single-precision%29))
  (Utilities|FlowControl|Sequence
    (:then_0
      (if (Variables|Default|GetEntering)
        (bind _output_get (Variables|/Script/Engine.PostProcessVolume|SetBlendWeight (Variables|Default|GetPP_Boost) (+ (Variables|Default|GetPP_Visibility) 0.1)))
        (Variables|Default|SetPP_Visibility _output_get)))
    (:then_1
      ;[0.15 0.15 0.15 0.5] Visibility_fade
      (if (Variables|Default|GetStopping)
        (bind _output_get_2 (Variables|/Script/Engine.PostProcessVolume|SetBlendWeight (Variables|Default|GetPP_Boost) (- (Variables|Default|GetPP_Visibility) 0.1)))
        (Variables|Default|SetPP_Visibility _output_get_2)))))

(fn ConstructionScript)