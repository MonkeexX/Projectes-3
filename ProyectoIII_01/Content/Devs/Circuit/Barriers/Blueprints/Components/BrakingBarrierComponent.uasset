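; Braking barrier component that penalises the player's Ship on overlap in the circuit game.
; A hit plays a sound and, unless a brake is already active, cuts SceneManager time, triggers the UIManager time-down, attaches a Niagara burst and nudges camera FOV.
; It lowers the ship's boost multiplier, restoring it after timed delays.
; Delay-toggled Entering and Exiting flags let Tick fade the debuff post-process in and out in fixed per-frame steps.
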(event Custom|On%20Overlap
  (params (Other%20Actor :type Actor%20Object%20Reference))
  (bind _as_ship (Variables|Default|GetAs%20Ship))
  (bind _as_scenemanager (Variables|Default|GetAs%20SceneManager))
  (bind _camera (Variables|/Game/Devs/Ship/Ship.Ship_C|GetCamera _as_ship))
  (if (== Other%20Actor (Variables|Default|GetAs%20Ship))
    (Audio|PlaySound2D "/Game/Devs/Circuit/Barriers/Sound/BreakBarrierSound.BreakBarrierSound" 1.0 1.0 0.0 0 0)
    (if (not (Variables|Default|GetBarrierBrake))
      (Utilities|FlowControl|Sequence
        (:then_0
          (Variables|/Game/Devs/Managers/SceneManager.SceneManager_C|SetTimeLeft _as_scenemanager (- (Variables|/Game/Devs/Managers/SceneManager.SceneManager_C|GetTimeLeft _as_scenemanager) 1e+01))
          (Variables|Default|SetBarrierBrake true)
          (bind _returnvalue (Niagara|SpawnSystemAttached "/Game/Artist/NS_VFX/NS_BarrierEx/NS_BarrierEx_S.NS_BarrierEx_S" (Variables|/Game/Devs/Ship/Ship.Ship_C|GetShip _as_ship) "Ship" "1000.000000,0.000000,0.000000" "0, 0, 0" "KeepRelativeOffset" true))
          (Utilities|FlowControl|Delay 1.0)
          (Components|DestroyComponent _returnvalue)
          (Variables|/Script/Engine.CameraComponent|SetFieldOfView _camera (Math|Interpolation|FInterpTo (Variables|/Script/Engine.CameraComponent|GetFieldOfView _camera) (- (Variables|/Script/Engine.CameraComponent|GetFieldOfView _camera) 15.0) (Utilities|Time|GetWorldDeltaSeconds) 0.0001))
          (Variables|/Game/Devs/Ship/Ship.Ship_C|SetBoostMult _as_ship (- (Variables|/Game/Devs/Ship/Ship.Ship_C|GetBoostMult _as_ship) 0.25))
          (Utilities|FlowControl|Delay 2.0)
          (Variables|/Game/Devs/Ship/Ship.Ship_C|SetBoostMult _as_ship (+ (Variables|/Game/Devs/Ship/Ship.Ship_C|GetBoostMult _as_ship) 0.25))
          (Variables|Default|SetBarrierBrake false))
        (:then_1
          (Variables|Default|SetEntering true)
          (Utilities|FlowControl|Delay 0.2)
          (Variables|Default|SetEntering false))
        (:then_2
          (Utilities|FlowControl|Delay 1.5)
          (Variables|Default|SetExiting true)
          (Utilities|FlowControl|Delay 0.5)
          (Variables|Default|SetExiting false))
        (:then_3
          (Default|TimeDown (Variables|Default|GetAs%20UIManager)))))))

(event EventBeginPlay
  (bind _returnvalue (Actor|GetActorOfClass "/Game/Devs/Ship/UIManager.UIManager_C"))
  (Variables|Default|SetAs%20UIManager _returnvalue)
  (bind _returnvalue_2 (Actor|GetActorOfClass "/Game/Devs/Managers/SceneManager.SceneManager_C"))
  (Variables|Default|SetAs%20SceneManager _returnvalue_2)
  (bind _asship (Utilities|Casting|CastToShip (Game|Player|GetPlayerPawn 0)))
  (Variables|Default|SetAs%20Ship _asship)
  (Variables|/Script/Engine.PostProcessVolume|SetBlendWeight (Variables|Default|GetPP_Boost) 0.0)
  (Variables|/Script/Engine.PostProcessVolume|SetBlendWeight (Variables|Default|GetPP_Debuff) 0.0))

(event EventTick
  (params (DeltaSeconds :type Float%20%28single-precision%29))
  (Utilities|FlowControl|Sequence
    (:then_0
      (if (Variables|Default|GetEntering)
        (bind _output_get (Variables|/Script/Engine.PostProcessVolume|SetBlendWeight (Variables|Default|GetPP_Debuff) (+ (Variables|Default|GetPP_Visibility) 0.15)))
        (Variables|Default|SetPP_Visibility _output_get)))
    (:then_1
      (if (Variables|Default|GetExiting)
        (bind _output_get_2 (Variables|/Script/Engine.PostProcessVolume|SetBlendWeight (Variables|Default|GetPP_Debuff) (- (Variables|Default|GetPP_Visibility) 0.15)))
        (Variables|Default|SetPP_Visibility _output_get_2)))))