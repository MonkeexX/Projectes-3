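; BP_GhostRunner is a ship Blueprint that drives boost effects from its mesh's movement and refills a boost meter.
; Each Tick compares the StaticMesh's world position with the previous one to set IsMoving.
; While moving, it shows BoostRed normally or BoostPurple after a short delay when IsBoosting, and deactivates both when still.
; Boost recharges per frame, unscaled by delta time, up to a cap while not boosting; IsBoosting is only read here.
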(event EventTick
  (params (DeltaSeconds :type Float%20%28single-precision%29))
  (Utilities|FlowControl|Sequence
    (:then_0
      (if (> (Math|Vector|Distance(Vector) (Variables|Default|GetLastPosition) (Transformation|GetWorldLocation (Variables|Default|GetStaticMesh))) 0.5)
        (Variables|Default|SetisMoving true)
        (else
          (Variables|Default|SetisMoving false)))
      (Variables|Default|SetLastPosition (Transformation|GetWorldLocation (Variables|Default|GetStaticMesh))))
    (:then_1
      ;[1 0.4177 0.8755 0.5] Boost_color
      (if (Variables|Default|GetIsMoving)
        (if (Variables|Default|GetisBoosting)
          (Utilities|FlowControl|Delay 0.2)
          (Components|Activation|Activate (Variables|Default|GetBoostPurple) false)
          (Components|Activation|Deactivate (Variables|Default|GetBoostRed))
          (else
            (Components|Activation|Activate (Variables|Default|GetBoostRed) false)
            (Components|Activation|Deactivate (Variables|Default|GetBoostPurple))))
        (else
          (Components|Activation|Deactivate (Variables|Default|GetBoostRed))
          (Components|Activation|Deactivate (Variables|Default|GetBoostPurple)))))
    (:then_2
      ;[0.1686 0.7708 0.4903 0.5] Boost
      (if (and (< (Variables|Default|GetBoost) 5e+02) (not (Variables|Default|GetisBoosting)))
        (Variables|Default|SetBoost (+ (Variables|Default|GetBoost) 0.4))))))

(fn ConstructionScript)