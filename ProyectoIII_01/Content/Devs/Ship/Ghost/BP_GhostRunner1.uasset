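; Ghost ship that replays a path of positions and rotations loaded from the GhostSave1 slot at BeginPlay.
; Each Tick, SetRotation and SetPosition step through the saved arrays with a shared Alpha that advances per frame, not by time, and position lerps with the saved point as A.
; Tick also toggles red or purple boost effects from movement and IsBoosting, and refills Boost.
; A BeginPlay loop creates an unused GhostSave object every 0.2 seconds.
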(event EventBeginPlay
  (bind _returnvalue (SaveGame|DoesSaveGameExist "GhostSave1" 1))
  (if _returnvalue
    (bind _returnvalue_2 (SaveGame|LoadGamefromSlot "GhostSave1" 1))
    (Variables|Default|SetObjectSave _returnvalue_2)
    (else
      (bind _returnvalue_3 (SaveGame|CreateSaveGameObject "/Game/Devs/Ship/Ghost/GhostSave.GhostSave_C"))
      (SaveGame|SaveGametoSlot _returnvalue_3 "GhostSave1" 1)
      (Variables|Default|SetObjectSave 0)))
  (CallFunction|ReadPositions)
  (CallFunction|ReadRotations)
  (bind _returnvalue_4 (SaveGame|CreateSaveGameObject "/Game/Devs/Ship/Ghost/GhostSave.GhostSave_C" :!label _label))
  (Variables|Default|SetSave _returnvalue_4)
  (Utilities|FlowControl|Delay 0.2)
  (goto _label))

(event EventTick
  (params (DeltaSeconds :type Float%20%28single-precision%29))
  (Utilities|FlowControl|Sequence
    (:then_0
      (if (> (Math|Vector|Distance(Vector) (Variables|Default|GetLastPosition) (Transformation|GetWorldLocation (Variables|Default|GetStaticMesh))) 0.5)
        (Variables|Default|SetisMoving true)
        (else
          (Variables|Default|SetisMoving false)))
      (Variables|Default|SetLastPosition (Transformation|GetWorldLocation (Variables|Default|GetStaticMesh))))
    (:then_1
      ;[1 0.4177 0.8755 0.5] Boost_color
      (if (Variables|Default|GetIsMoving)
        (if (Variables|Default|GetisBoosting)
          (Utilities|FlowControl|Delay 0.2)
          (Components|Activation|Activate (Variables|Default|GetBoostPurple) false)
          (Components|Activation|Deactivate (Variables|Default|GetBoostRed))
          (else
            (Components|Activation|Activate (Variables|Default|GetBoostRed) false)
            (Components|Activation|Deactivate (Variables|Default|GetBoostPurple))))
        (else
          (Components|Activation|Deactivate (Variables|Default|GetBoostRed))
          (Components|Activation|Deactivate (Variables|Default|GetBoostPurple)))))
    (:then_2
      ;[0.1686 0.7708 0.4903 0.5] Boost
      (if (and (< (Variables|Default|GetBoost) 5e+02) (not (Variables|Default|GetisBoosting)))
        (Variables|Default|SetBoost (+ (Variables|Default|GetBoost) 0.4))))
    (:then_3
      (CallFunction|SetRotation)
      (CallFunction|SetPosition))))

(fn ConstructionScript)

(fn ReadPositions
  (bind _asghost_save (Utilities|Casting|CastToGhostSave (Variables|Default|GetObjectSave)))
  (Variables|Default|SetPositions (Variables|/Game/Devs/Ship/Ghost/GhostSave.GhostSave_C|Getsavedpos _asghost_save)))

(fn ReadRotations
  (bind _asghost_save (Utilities|Casting|CastToGhostSave (Variables|Default|GetObjectSave)))
  (Variables|Default|SetRotations (Variables|/Game/Devs/Ship/Ghost/GhostSave.GhostSave_C|GetsavedRotation _asghost_save)))

(fn SetPosition
  (if (Variables|Default|GetFinishedMovingToPoint)
    (Variables|Default|Setalpha 0.0)
    (Variables|Default|SetFinishedMovingToPoint false)
    (bind _output_get (Variables|Default|SetStartingTime (Utilities|Time|GetGameTimeinSeconds)))
    (Variables|Default|SetFinishingTime (+ _output_get 0.15))
    (Variables|Default|SetCurrentPosition (Transformation|GetWorldLocation (Variables|Default|GetStaticMesh))))
  (Variables|Default|SetCurrentTime (Utilities|Time|GetGameTimeinSeconds))
  (if (>= 0.9 (Variables|Default|Getalpha))
    (if (> (Utilities|Array|Length (Variables|Default|GetPositions)) (Variables|Default|Getindex))
      (Development|PrintString (Utilities|String|ToString(Float) 0.0))
      (Transformation|SetWorldLocation (Variables|Default|GetStaticMesh) (Math|Vector|Lerp(Vector) (Utilities|Array|Get(acopy) (Variables|Default|GetPositions) (Variables|Default|Getindex)) (Transformation|GetWorldLocation (Variables|Default|GetStaticMesh)) (Variables|Default|Getalpha)) false false))
    (else
      (Variables|Default|SetFinishedMovingToPoint true)
      (Math|Integer|IncrementInt (Variables|Default|Getindex)
        (:%20%20
          (Variables|Default|Setalpha 0.0))))))

(fn SetRotation
  (if (Variables|Default|GetFinishedMovingToPoint)
    (Variables|Default|Setalpha 0.0)
    (Variables|Default|SetFinishedMovingToPoint false)
    (bind _output_get (Variables|Default|SetStartingTime (Utilities|Time|GetGameTimeinSeconds)))
    (Variables|Default|SetFinishingTime (+ _output_get 0.15)))
  (Variables|Default|SetCurrentTime (Utilities|Time|GetGameTimeinSeconds))
  (if (> (Utilities|Array|Length (Variables|Default|GetRotations)) (Variables|Default|Getindex))
    (bind _output_get_2 (Variables|Default|Setalpha (+ (Variables|Default|Getalpha) 0.13)))
    (Transformation|SetWorldRotation (Variables|Default|GetStaticMesh) (Math|Rotator|Lerp(Rotator) (Transformation|GetWorldRotation (Variables|Default|GetStaticMesh)) (Utilities|Array|Get(acopy) (Variables|Default|GetRotations) (Variables|Default|Getindex)) _output_get_2) false false)))