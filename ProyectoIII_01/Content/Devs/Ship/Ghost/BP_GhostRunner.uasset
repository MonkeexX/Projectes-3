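; Ghost ship that replays a saved run in the Holo and Factory District levels, destroying itself when the recording ends.
; BeginPlay picks the GhostSave slot by level name and loads recorded positions, rotations and times.
; Tick applies one sample per frame, ignoring the times, and switches red or purple thruster effects from recorded moving and boosting flags.
; BeginPlay also recreates an unused save object every 0.2 seconds.
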(event EventBeginPlay
  (CallFunction|GetNameSave)
  (bind _returnvalue (SaveGame|LoadGamefromSlot (Variables|Default|GetSaveDataName)))
  (Utilities|IsValid _returnvalue
    (:Is%20Valid
      (Variables|Default|SetNewVar_1 _returnvalue))
    (:Is%20Not%20Valid
      (bind _returnvalue_2 (SaveGame|CreateSaveGameObject "/Game/Devs/Ship/Ghost/GhostSave.GhostSave_C"))
      (Variables|Default|SetNewVar_1 _returnvalue_2)))
  (CallFunction|ReadPositions)
  (CallFunction|ReadRotations)
  (CallFunction|ReadTimes)
  (bind _returnvalue_3 (SaveGame|CreateSaveGameObject "/Game/Devs/Ship/Ghost/GhostSave.GhostSave_C" :!label _label))
  (Variables|Default|SetSave _returnvalue_3)
  (Utilities|FlowControl|Delay 0.2)
  (goto _label))

(event EventTick
  (params (DeltaSeconds :type Float%20%28single-precision%29))
  (CallFunction|SetPlacement)
  (if (< (- (Utilities|Array|Length (Variables|Default|GetRotations)) 1) (Variables|Default|Getindex))
    (Actor|DestroyActor)
    (else
      (CallFunction|SetRotation)
      (CallFunction|SetPosition)
      (CallFunction|ReadMovingandBoost)
      (CallFunction|IndexIncrement)
      (Utilities|FlowControl|Sequence
        (:then_0
          (if (> (Math|Vector|Distance(Vector) (Variables|Default|GetLastPosition) (Transformation|GetWorldLocation (Variables|Default|GetStaticMesh))) 0.5)
            (Variables|Default|SetisMoving true)
            (else
              (Variables|Default|SetisMoving false)))
          (Variables|Default|SetLastPosition (Transformation|GetWorldLocation (Variables|Default|GetStaticMesh))))
        (:then_1
          (CallFunction|GetItsMovingorBoosting)
          ;[1 0.4177 0.8755 0.5] Boost_color
          (if (Variables|Default|GetIsMoving)
            (if (Variables|Default|GetisBoosting)
              (Utilities|FlowControl|Delay 0.2)
              (Components|Activation|Activate (Variables|Default|GetBoostPurple) false)
              (Components|Activation|Deactivate (Variables|Default|GetBoostRed))
              (else
                (Components|Activation|Activate (Variables|Default|GetBoostRed) false)
                (Components|Activation|Deactivate (Variables|Default|GetBoostPurple))))
            (else
              (Components|Activation|Deactivate (Variables|Default|GetBoostRed))
              (Components|Activation|Deactivate (Variables|Default|GetBoostPurple)))))
        (:then_2
          ;[0.1686 0.7708 0.4903 0.5] Boost
          (if (and (< (Variables|Default|GetBoost) 5e+02) (not (Variables|Default|GetisBoosting)))
            (Variables|Default|SetBoost (+ (Variables|Default|GetBoost) 0.4))))))))

(fn ConstructionScript)

(fn ReadPositions
  (bind _asghost_save (Utilities|Casting|CastToGhostSave (Variables|Default|GetNewVar_1)))
  (Variables|Default|SetPositions (Variables|/Game/Devs/Ship/Ghost/GhostSave.GhostSave_C|Getsavedpos _asghost_save)))

(fn ReadTimes
  (bind _asghost_save (Utilities|Casting|CastToGhostSave (Variables|Default|GetNewVar_1)))
  (Variables|Default|SetTimes (Variables|/Game/Devs/Ship/Ghost/GhostSave.GhostSave_C|GetsavedTimes _asghost_save)))

(fn ReadMovingandBoost
  (bind _asghost_save (Utilities|Casting|CastToGhostSave (Variables|Default|GetNewVar_1)))
  (Variables|Default|SetBoosting (Variables|/Game/Devs/Ship/Ghost/GhostSave.GhostSave_C|GetsavedBoosting _asghost_save))
  (Variables|Default|SetMoving (Variables|/Game/Devs/Ship/Ghost/GhostSave.GhostSave_C|GetsavedMoving _asghost_save)))

(fn ReadRotations
  (bind _asghost_save (Utilities|Casting|CastToGhostSave (Variables|Default|GetNewVar_1)))
  (Variables|Default|SetRotations (Variables|/Game/Devs/Ship/Ghost/GhostSave.GhostSave_C|GetsavedRotation _asghost_save)))

(fn SetRotation
  (Transformation|SetWorldRotation (Variables|Default|GetStaticMesh) (Utilities|Array|Get(acopy) (Variables|Default|GetRotations) (Variables|Default|Getindex)) false false))

(fn SetPosition
  (Transformation|SetWorldLocation (Variables|Default|GetStaticMesh) (Utilities|Array|Get(acopy) (Variables|Default|GetPositions) (Variables|Default|Getindex)) false false))

(fn IndexIncrement
  (Math|Integer|IncrementInt (Variables|Default|Getindex)))

(fn GetItsMovingorBoosting
  (if (not (< (- (Utilities|Array|Length (Variables|Default|GetBoosting)) 1) (Variables|Default|Getindex)))
    (Variables|Default|SetisBoosting (Utilities|Array|Get(acopy) (Variables|Default|GetBoosting) (Variables|Default|Getindex)))
    (Variables|Default|SetisMoving (Utilities|Array|Get(acopy) (Variables|Default|GetMoving) (Variables|Default|Getindex)))))

(fn GetNameSave
  (bind _returnvalue (Game|GetCurrentLevelName true))
  (if (Utilities|Enum|Equal(Enum) _returnvalue "NC_HoloDistrict")
    (Variables|Default|SetSaveDataName "GhostSaveHoloDistrict")
    (SaveGame|LoadGamefromSlot (Variables|Default|GetSaveDataName) :!label _label)
    (Development|PrintString (Variables|Default|GetSaveDataName))
    (elif (Utilities|Enum|Equal(Enum) _returnvalue "NC_FactoryDistrict")
      (Variables|Default|SetSaveDataName "GhostSaveFactory")
      (goto _label))))

(fn SetPlacement
  (bind _outactors (Actor|GetAllActorsOfClass "/Game/Devs/Circuit/Checkpoint.Checkpoint_C"))
  (for _array_element _outactors
    (if (== (Variables|/Game/Devs/Circuit/Checkpoint.Checkpoint_C|GetPosition _array_element) (+ (Variables|Default|GetCheckPoint) 1))
      (Variables|Default|SetSavePoint (Transformation|GetWorldLocation (Variables|/Script/Engine.Actor|GetRootComponent _array_element))))))